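; BP_Player is the player Blueprint, setting up a pair of arms and tracking which arm action the input selects.
; On BeginPlay it casts two child actors to BSArmComponent, stores them in ArmArray and links each as the other's reverse arm.
; Holding Block, Grab or Reload sets CurrentArmInputType, and releasing restores AttackUse only if that mode is still current.
; The graph only sets this state and does not perform the actions.
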(event `self.ReceiveBeginPlay`
  (bind _armcomponents (`self.ArmComponents`))
  (bind _asbsarm_component_c (cast `BSArmComponent_C` (`ChildActorComponent.ChildActor` (`self.BP_PLARMV2`))))
  (`KismetArrayLibrary.Array_Add` _armcomponents _asbsarm_component_c)
  (bind _asbsarm_component_c_2 (cast `BSArmComponent_C` (`ChildActorComponent.ChildActor` (`self.BP_PLARMV3`))))
  (`KismetArrayLibrary.Array_Add` _armcomponents _asbsarm_component_c_2)
  (bind _output_get (set `self.ArmArray` _armcomponents))
  (bind _output (`|GetArrayItem` _output_get))
  (bind _output_2 (`|GetArrayItem` _output_get 1))
  (`BSArmComponent_C.SetReverseArmComponent` _output _output_2)
  (`BSArmComponent_C.SetReverseArmComponent` _output_2 _output))

(event `self.ReceiveTick`
  (params (DeltaSeconds :type "Float (single-precision)")))

(event `self.TickV2`
  (params (DeltaTime :type "Float (single-precision)")))

(event `EnhancedInput|/Game/Input/IA_ARM_Block`
  (params (ActionValue :type Boolean) (ElapsedSeconds :type "Float (double-precision)") (TriggeredSeconds :type "Float (double-precision)") (InputAction :type "InputAction Object Reference" :default "/Game/Input/IA_ARM_Block.IA_ARM_Block"))
  (:`Started`
    (set `self.CurrentArmInputType` "Block"))
  (:`Completed`
    (if (`|EnumEquality` (`self.CurrentArmInputType`) "Block")
      (set `self.CurrentArmInputType` "AttackUse" :!label _label))))

(event `EnhancedInput|/Game/Input/IA_ARM_Grab`
  (params (ActionValue :type Boolean) (ElapsedSeconds :type "Float (double-precision)") (TriggeredSeconds :type "Float (double-precision)") (InputAction :type "InputAction Object Reference" :default "/Game/Input/IA_ARM_Grab.IA_ARM_Grab"))
  (:`Started`
    (set `self.CurrentArmInputType` "Grab"))
  (:`Completed`
    (if (`|EnumEquality` (`self.CurrentArmInputType`) "Grab")
      (goto _label))))

(event `EnhancedInput|/Game/Input/IA_ARM_Reload`
  (params (ActionValue :type Boolean) (ElapsedSeconds :type "Float (double-precision)") (TriggeredSeconds :type "Float (double-precision)") (InputAction :type "InputAction Object Reference" :default "/Game/Input/IA_ARM_Reload.IA_ARM_Reload"))
  (:`Started`
    (set `self.CurrentArmInputType` "Reload"))
  (:`Completed`
    (if (`|EnumEquality` (`self.CurrentArmInputType`) "Reload")
      (goto _label))))

(fn `UserConstructionScript`)