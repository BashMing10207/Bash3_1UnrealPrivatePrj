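; BP_Cow1 is a cow entity that chases its Target, or the player pawn if none is valid, and drops food on death.
; A looping timer runs Move, which feeds that location to PathFinder and stores the result as InputVector.
; TickV2 drives BSBashMovement with that vector and sets controller yaw to match.
; Damage reduces HP, and at zero it spawns BP_FOOD1 and destroys itself.
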(event `self.ReceiveBeginPlay`
  (`KismetSystemLibrary.K2_SetTimerDelegate` (delegate `CustomEvent`) 0.1 true))

(event `CustomEvent`
  (`self.Move`))

(event `self.TickV2`
  (params (DeltaTime :type "Float (single-precision)"))
  (bind _inputvector (`self.InputVector`))
  (bind _bsbashmovement (`self.BSBashMovement`))
  (bind (_returnvalue_roll _returnvalue_pitch _returnvalue_yaw) (`KismetMathLibrary.BreakRotator` (`KismetMathLibrary.Conv_VectorToRotator` _inputvector)))
  (`BSBashMovement.Movement` _bsbashmovement DeltaTime _inputvector (`BSBashMovement.MaxSpeed` _bsbashmovement) (`BSBashMovement.Accelation` _bsbashmovement))
  (`Controller.SetControlRotation` (`self.GetController`) (`KismetMathLibrary.MakeRotator` 0.0 0.0 _returnvalue_yaw)))

(event `self.ReceiveAnyDamage`
  (params (Damage :type "Float (single-precision)") (DamageType :type "DamageType Object Reference") (InstigatedBy :type "Controller Object Reference") (DamageCauser :type "Actor Object Reference"))
  (bind _output_get (set `self.HP` (- (`self.HP`) Damage)))
  (if (<= _output_get 0.0)
    (`|SpawnActorFromClass` "/Game/00_BP/Item/BP_FOOD1.BP_FOOD1_C" (`SceneComponent.K2_GetComponentToWorld` (`self.BaseBodyCompo`)) "AlwaysSpawn" "MultiplyWithRoot" null null)
    (`self.K2_DestroyActor`)))

(fn `Move`
  (bind _pathfinder (`self.PathFinder`))
  (bind _target (`self.Target`))
  (if (`KismetSystemLibrary.IsValid` _target)
    (set `PTBashAI.MyTargetLocation` (`self.K2_GetActorLocation` _target) _pathfinder)
    (else
      (set `PTBashAI.MyTargetLocation` (`self.K2_GetActorLocation` (`GameplayStatics.GetPlayerPawn` 0)) _pathfinder)))
  (bind _returnvalue (`PTBashAI.BashPathFind` _pathfinder))
  (set `self.InputVector` _returnvalue))

(fn `NewFunction`)

(fn `UserConstructionScript`)