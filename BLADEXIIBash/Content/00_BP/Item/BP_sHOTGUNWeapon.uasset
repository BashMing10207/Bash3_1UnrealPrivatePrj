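; Shotgun weapon item that fires a spread of spawned actors from its mesh's Muzzle socket when used.
; RealUseItemObj spawns one actor per entry in Dir, each stretched along X and rotated off the muzzle direction by random roll, pitch and yaw from NewFunction.
; Each shot costs one Ammo; once it falls below zero, the using arm drops the item and the weapon destroys itself.
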(fn `NewFunction`
  (returns (ReturnValue :type "Float (double-precision)") (NewParam :type "Float (double-precision)") (NewParam1 :type "Float (double-precision)"))
  (return (`KismetMathLibrary.RandomFloatInRange` -8.0 8.0) (`KismetMathLibrary.RandomFloatInRange` -8.0 8.0) (`KismetMathLibrary.RandomFloatInRange` -8.0 8.0)))

(fn `RealUseItemObj`
  (params (UsingArm :type "BSArmComponent_C Object Reference") (Caller :type "Actor Object Reference"))
  (returns (ReturnValue :type "BSItemObjBase Object Reference"))
  (bind (_returnvalue_location _returnvalue_rotation) (`KismetMathLibrary.BreakTransform` (`SceneComponent.GetSocketTransform` (`self.MeshCompo`) "Muzzle" "RTS_World")))
  (for _ (`self.Dir`)
    (bind (_returnvalue _newparam _newparam1) (`self.NewFunction`))
    (`|SpawnActorFromClass` (`self.NewVar`) (`KismetMathLibrary.MakeTransform` _returnvalue_location (`KismetMathLibrary.ComposeRotators` (`KismetMathLibrary.MakeRotator` _returnvalue _newparam _newparam1) _returnvalue_rotation) (3.0 1.0 1.0)) "AlwaysSpawn" "MultiplyWithRoot" null null))
  (bind _output_get (set `self.Ammo` (- (`self.Ammo`) 1)))
  (if (< _output_get 0)
    (`BSArmComponent_C.DropItem` UsingArm)
    (`self.K2_DestroyActor`))
  (return null))

(fn `UserConstructionScript`)