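; BP_MeleeWeapon is a usable melee weapon item that damages actors it overlaps while in an attacking state.
; RealUseItemObj stores the caller and using arm as owners and toggles IsAttacking on each use.
; While attacking, every begin-overlap with an actor other than those two owners applies the weapon's Damage as environmental damage, crediting the owning actor as damage causer.
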(event `self.ReceiveActorBeginOverlap`
  (params (OtherActor :type "Actor Object Reference"))
  (bind _owningactor (`self.OwningActor`))
  (if (and (!= OtherActor _owningactor) (!= OtherActor (`self.OwningArm`)) (`self.IsAttacking`))
    (`GameplayStatics.ApplyDamage` OtherActor (`self.Damage`) null _owningactor "/Engine/EngineDamageTypes/DmgTypeBP_Environmental.DmgTypeBP_Environmental_C")))

(fn `RealUseItemObj`
  (params (UsingArm :type "BSArmComponent_C Object Reference") (Caller :type "Actor Object Reference"))
  (returns (ReturnValue :type "BSItemObjBase Object Reference"))
  (set `self.OwningActor` Caller)
  (set `self.OwningArm` UsingArm)
  (set `self.IsAttacking` (not (`self.IsAttacking`)))
  (return null))

(fn `UserConstructionScript`)