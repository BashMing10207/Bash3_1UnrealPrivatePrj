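; BP_GAS is a moving gas hazard actor that affects BP_Player while the player is inside it.
; Player overlap with the actor enables its PostProcess and sets the player's ISGAS flag; ending overlap with the Cube component clears both.
; Tick teleports the actor along world +Y at a constant, delta-time-scaled speed.
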(event `self.ReceiveActorBeginOverlap`
  (params (OtherActor :type "Actor Object Reference"))
  (bind _asbp_player (cast `/Game/00_BP/ENtity/Player/BP_Player` OtherActor))
  (set `PostProcessComponent.bEnabled` true (`self.PostProcess`))
  (set `/Game/00_BP/ENtity/Player/BP_Player.ISGAS` true _asbp_player))

(event `self.Cube.OnComponentEndOverlap`
  (params (OverlappedComponent :type "PrimitiveComponent Object Reference") (OtherActor :type "Actor Object Reference") (OtherComp :type "PrimitiveComponent Object Reference") (OtherBodyIndex :type Integer))
  (bind _asbp_player (cast `/Game/00_BP/ENtity/Player/BP_Player` OtherActor))
  (set `PostProcessComponent.bEnabled` false (`self.PostProcess`))
  (set `/Game/00_BP/ENtity/Player/BP_Player.ISGAS` false _asbp_player))

(event `self.ReceiveTick`
  (params (DeltaSeconds :type "Float (single-precision)"))
  (bind (_returnvalue_x _returnvalue_y _returnvalue_z) (`KismetMathLibrary.BreakVector` (`self.K2_GetActorLocation`)))
  (`self.K2_SetActorLocation` (`KismetMathLibrary.MakeVector` _returnvalue_x (+ _returnvalue_y (* DeltaSeconds 60.0)) _returnvalue_z) false true))

(fn `UserConstructionScript`)