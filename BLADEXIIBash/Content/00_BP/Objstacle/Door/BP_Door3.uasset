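; BP_Door3 is an obstacle door that opens through damage, a key or direct interaction.
; Damage drains HP until it reaches zero; UseKey accepts Id 1, and DOInteractive checks that Opened is false.
; All three routes call OPEN, which only spawns a configurable actor class at the Scene transform, without setting Opened.
; Tick continuously rotates the Steak2 component, while morph-target damage feedback and DestroyActor are left disconnected.
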(event `self.ReceiveTick`
  (params (DeltaSeconds :type "Float (single-precision)"))
  (`SceneComponent.K2_AddRelativeRotation` (`self.Steak_2`) (struct :`Yaw` 1.0) false false))

(event `self.ReceiveAnyDamage`
  (params (Damage :type "Float (single-precision)") (DamageType :type "DamageType Object Reference") (InstigatedBy :type "Controller Object Reference") (DamageCauser :type "Actor Object Reference"))
  (bind _output_get (set `self.HP` (- (`self.HP`) Damage)))
  (if (<= _output_get 0.0)
    (`self.OPEN`)))

(fn `DOInteractive`
  (params (UsingArm :type "BSArmComponent_C Object Reference") (Caller :type "Actor Object Reference"))
  (returns (ReturnValue :type "BSItemObjBase Object Reference"))
  (if (not (`self.Opened`))
    (`self.OPEN`)
    (return null)))

(fn `OPEN`
  (`|SpawnActorFromClass` (`self.class`) (`SceneComponent.K2_GetComponentToWorld` (`self.Scene`)) "Undefined" "MultiplyWithRoot" null null))

(fn `UseKey`
  (params (id :type Integer))
  (returns (ReturnValue :type "Actor Object Reference"))
  (if (== id 1)
    (`self.OPEN`)
    (return self)))

(fn `UserConstructionScript`)