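; BP_Door is a breakable door obstacle that opens by switching to physics simulation and being shoved along the actor's forward vector.
; Interaction opens it unless Opened is set, and UseKey opens it for key Id zero.
; Damage drains HP, and at zero or below the door opens with an extra force scaled by BreakAdd.
; OPEN never sets Opened, and the morph-target damage and DestroyActor nodes are disconnected.
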(event `self.ReceiveAnyDamage`
  (params (Damage :type "Float (single-precision)") (DamageType :type "DamageType Object Reference") (InstigatedBy :type "Controller Object Reference") (DamageCauser :type "Actor Object Reference"))
  (bind _output_get (set `self.HP` (- (`self.HP`) Damage)))
  (if (<= _output_get 0.0)
    (`self.OPEN`)
    (`PrimitiveComponent.AddForce` (`self.Door`) (* (* (`self.GetActorForwardVector`) (`self.Power`)) (`self.Break Add`)) "None" true)))

(fn `DOInteractive`
  (params (UsingArm :type "BSArmComponent_C Object Reference") (Caller :type "Actor Object Reference"))
  (returns (ReturnValue :type "BSItemObjBase Object Reference"))
  (if (not (`self.Opened`))
    (`self.OPEN`)
    (return null)))

(fn `OPEN`
  (bind _door (`self.Door`))
  (`PrimitiveComponent.SetSimulatePhysics` _door true)
  (`PrimitiveComponent.AddForce` _door (* (`self.GetActorForwardVector`) (`self.Power`)) "None" true))

(fn `UseKey`
  (params (id :type Integer))
  (returns (ReturnValue :type "Actor Object Reference"))
  (if (== id 0)
    (`self.OPEN`)
    (return null)))

(fn `UserConstructionScript`)